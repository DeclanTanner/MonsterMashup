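; BP_Held1 is a rhythm-game hold note that travels along a lane spline, with upper and lower flipbook variants.
; Tick places the head and a tail delayed by the hold duration, stretching and rotating a trail sprite between them.
; StartHold, ReleaseHold and CompleteHold track the press, allowing a slightly early release and dimming broken notes.
; Outcomes go to BP_Spline as judgements, and notes are destroyed on completion or when the tail reaches the lane's end.
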(event `self.ReceiveBeginPlay`
  (bind _isupper (`self.IsUpper`))
  (bind _returnvalue (`GameplayStatics.GetActorOfClass` "/Game/Mash/Blueprints/BP_Spline.BP_Spline_C"))
  (set `self.RythmSpline` _returnvalue)
  (`PaperFlipbookComponent.SetFlipbook` (`self.EnemySprite`) (select `bool` _isupper :`false` (`self.BottomHold`) :`true` (`self.TopHold`)))
  (`PaperFlipbookComponent.SetFlipbook` (`self.EnemySpriteTail`) (select `bool` _isupper :`false` (`self.BottomHoldHit`) :`true` (`self.TopHoldHit`))))

(event `self.ReceiveTick`
  (params (DeltaSeconds :type "Float (single-precision)"))
  (bind _returnvalue (`self.K2_GetActorLocation`))
  (bind _returnvalue_2 (`SplineComponent.GetSplineLength` (`self.Lane`)))
  (bind _returnvalue_3 (`SplineComponent.GetLocationAtDistanceAlongSpline` (`self.Lane`) (`KismetMathLibrary.FClamp` (* (- (`self.Elapsed`) (`self.HoldDuration`)) (`self.GetSpeed`)) 0.0 (`SplineComponent.GetSplineLength` (`self.Lane`))) "World"))
  (set `self.Elapsed` (+ (`self.Elapsed`) DeltaSeconds))
  (`self.K2_SetActorLocation` (`SplineComponent.GetLocationAtDistanceAlongSpline` (`self.Lane`) (`KismetMathLibrary.FClamp` (* (`self.Elapsed`) (`self.GetSpeed`)) 0.0 (`SplineComponent.GetSplineLength` (`self.Lane`))) "World"))
  (`SceneComponent.K2_SetWorldLocation` (`self.EnemySpriteTail`) (+ _returnvalue_3 (0.0 0.0 10.0)) false false)
  (`SceneComponent.K2_SetWorldLocation` (`self.TrailSprite`) (/ (+ (`self.K2_GetActorLocation`) _returnvalue_3) 2.0) false false)
  (`SceneComponent.K2_SetWorldRotation` (`self.TrailSprite`) (`KismetMathLibrary.FindLookAtRotation` _returnvalue_3 _returnvalue) false false)
  (`SceneComponent.SetWorldScale3D` (`self.TrailSprite`) (`KismetMathLibrary.MakeVector` (/ (`KismetMathLibrary.Vector_Distance` _returnvalue _returnvalue_3) 2048.0) 0.1 0.1))
  (if (and (`self.Holding`) (>= (- (`self.Elapsed`) (`self.PressTime`)) (`self.HoldDuration`)))
    (`self.CompleteHold`)
    (elif (>= (`KismetMathLibrary.FClamp` (* (- (`self.Elapsed`) (`self.HoldDuration`)) (`self.GetSpeed`)) 0.0 _returnvalue_2) _returnvalue_2)
      (if (not (`self.Judged`))
        (`/Game/Mash/Blueprints/BP_Spline.ApplyJudgement` (`self.RythmSpline`) "NewEnumerator4"))
      (`self.K2_DestroyActor`))))

(fn `CompleteHold`
  (set `self.Holding` false)
  (`/Game/Mash/Blueprints/BP_Spline.ApplyJudgement` (`self.RythmSpline`) "NewEnumerator3")
  (`self.K2_DestroyActor`))

(fn `ReleaseHold`
  (if (`self.Holding`)
    (if (<= (- (`self.HoldDuration`) (- (`self.Elapsed`) (`self.PressTime`))) 0.15)
      (`self.CompleteHold`)
      (else
        (set `self.Holding` false)
        (set `self.Broken` true)
        (`PaperFlipbookComponent.SetFlipbook` (`self.EnemySprite`) (select `bool` (`self.IsUpper`) :`false` (`self.BottomHold`) :`true` (`self.TopHold`)))
        (`PaperFlipbookComponent.SetSpriteColor` (`self.EnemySprite`) (struct :`R` 0.223958 :`G` 0.223958 :`B` 0.223958 :`A` 1.0))
        (`/Game/Mash/Blueprints/BP_Spline.ApplyJudgement` (`self.RythmSpline`) "NewEnumerator4")))))

(fn `StartHold`
  (`PaperFlipbookComponent.SetFlipbook` (`self.EnemySprite`) (select `bool` (`self.IsUpper`) :`false` (`self.BottomHoldHit`) :`true` (`self.TopHoldHit`)))
  (set `self.Holding` true)
  (set `self.PressTime` (`self.Elapsed`)))

(fn `UserConstructionScript`
  (`parent.UserConstructionScript`))