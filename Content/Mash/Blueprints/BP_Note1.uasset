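; BP_Note1 is a rhythm note shown as an animated enemy sprite, with top or bottom flipbooks chosen by IsUpper.
; On BeginPlay it follows the Lane spline's position and rotation through a Timeline scaled to finish in TimeToComplete.
; PlayHit marks it judged, stops movement and collision, shows the hit flipbook and destroys it after a short delay.
; GetSpeed returns spline length over travel time.
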(event `self.ReceiveBeginPlay`
  (`PaperFlipbookComponent.SetFlipbook` (`self.EnemySprite`) (select `bool` (`self.IsUpper`) :`false` (`self.BottomRun`) :`true` (`self.TopRun`)))
  (`self.MoveNotes`))

(event `PlayHit`
  (set `self.Judged` true)
  (`TimelineComponent.Stop` (`self.Timeline`))
  (`PrimitiveComponent.SetCollisionEnabled` (`self.Sphere`) "NoCollision")
  (`PaperFlipbookComponent.SetFlipbook` (`self.EnemySprite`) (select `bool` (`self.IsUpper`) :`false` (`self.BottomHit`) :`true` (`self.TopHit`)))
  (`KismetSystemLibrary.Delay` 0.2)
  (`self.K2_DestroyActor`))

(event `MoveNotes`
  (bind _lane (`self.Lane`))
  ;[1 1 1] Move Along Track
  (`TimelineComponent.SetPlayRate` (`self.Timeline`) (/ 1.0 (`self.TimeToComplete`)))
  (bind (_direction _newtrack_0) (`Timeline|Timeline` :!via `PlayFromStart`)
    (:`Update`
      (bind _returnvalue (`KismetMathLibrary.Lerp` 0.0 (`SplineComponent.GetSplineLength` (`self.Lane`)) _newtrack_0))
      (`self.K2_SetActorTransform` (`KismetMathLibrary.MakeTransform` (`SplineComponent.GetLocationAtDistanceAlongSpline` _lane _returnvalue "World") (`SplineComponent.GetRotationAtDistanceAlongSpline` _lane _returnvalue "World") (`SceneComponent.RelativeScale3D` (`self.Sphere`)))))))

(fn `GetSpeed`
  (returns (Speed :type "Float (double-precision)"))
  (return (/ (`SplineComponent.GetSplineLength` (`self.Lane`)) (`self.TimeToComplete`))))

(fn `UserConstructionScript`)