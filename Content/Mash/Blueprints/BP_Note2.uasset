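; BP_Note2 is a rhythm-game note actor that travels along the lower lane of the level's BP_Spline.
; It finds the spline actor on BeginPlay.
; MoveNotesLower plays a timeline, rate-scaled by TimeToComplete, that maps its alpha to spline distance and sets location and rotation, applying the Sphere's relative scale.
; GetSpeed divides the upper lane's length by TimeToComplete, although movement follows the lower lane.
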(event `self.ReceiveBeginPlay`
  (bind _returnvalue (`GameplayStatics.GetActorOfClass` "/Game/Mash/Blueprints/BP_Spline.BP_Spline_C"))
  (set `self.RythmSpline` _returnvalue))

(event `MoveNotesLower`
  (bind _lanelower (`/Game/Mash/Blueprints/BP_Spline.LaneLower` (`self.RythmSpline`)))
  ;[1 1 1] Move Along Track
  (`TimelineComponent.SetPlayRate` (`self.Timeline`) (/ 1.0 (`self.TimeToComplete`)))
  (bind (_direction _newtrack_0) (`Timeline|Timeline` :!via `PlayFromStart`)
    (:`Update`
      (bind _returnvalue (`KismetMathLibrary.Lerp` 0.0 (`SplineComponent.GetSplineLength` (`/Game/Mash/Blueprints/BP_Spline.LaneLower` (`self.RythmSpline`))) _newtrack_0))
      (`self.K2_SetActorTransform` (`KismetMathLibrary.MakeTransform` (`SplineComponent.GetLocationAtDistanceAlongSpline` _lanelower _returnvalue "World") (`SplineComponent.GetRotationAtDistanceAlongSpline` _lanelower _returnvalue "World") (`SceneComponent.RelativeScale3D` (`self.Sphere`)))))))

(fn `GetSpeed`
  (returns (Speed :type "Float (double-precision)"))
  (return (/ (`SplineComponent.GetSplineLength` (`/Game/Mash/Blueprints/BP_Spline.LaneUpper` (`self.RythmSpline`))) (`self.TimeToComplete`))))

(fn `UserConstructionScript`)